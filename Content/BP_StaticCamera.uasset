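; BP_StaticCamera is an actor that takes over the player's view while the player character overlaps it, acting as a fixed camera zone.
; On begin overlap it stores the current view target, then blends the player controller's view to itself over a short time.
; On end overlap it blends back to the stored previous view target.
; Both events respond only to the first player's character.
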(event `self.ReceiveActorBeginOverlap`
  (params (OtherActor :type "Actor Object Reference"))
  (bind _returnvalue (`GameplayStatics.GetPlayerController` 0))
  (if (== OtherActor (`GameplayStatics.GetPlayerCharacter` 0))
    (set `self.PreviousCamera` (`Controller.GetViewTarget` _returnvalue))
    (`PlayerController.SetViewTargetWithBlend` _returnvalue self 0.5 "VTBlend_Linear" 0.0 false)))

(event `self.ReceiveActorEndOverlap`
  (params (OtherActor :type "Actor Object Reference"))
  (if (== OtherActor (`GameplayStatics.GetPlayerCharacter` 0))
    (`PlayerController.SetViewTargetWithBlend` (`GameplayStatics.GetPlayerController` 0) (`self.PreviousCamera`) 0.5 "VTBlend_Linear" 0.0 false)))

(fn `UserConstructionScript`)