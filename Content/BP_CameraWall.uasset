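; BP_CameraWall is an overlap actor that applies a camera effect while the player character is inside it.
; On begin overlap with the player character, it adds a CM_FOV modifier to the player camera manager and stores the instance in CM.
; On end overlap, it removes that stored modifier, so the effect lasts only for the duration of the overlap.
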(event `self.ReceiveActorBeginOverlap`
  (params (OtherActor :type "Actor Object Reference"))
  (if (== OtherActor (`GameplayStatics.GetPlayerCharacter` 0))
    (bind _returnvalue (`PlayerCameraManager.AddNewCameraModifier` (`GameplayStatics.GetPlayerCameraManager` 0) "/Game/CM_FOV.CM_FOV_C"))
    (set `self.CM` _returnvalue)))

(event `self.ReceiveActorEndOverlap`
  (params (OtherActor :type "Actor Object Reference"))
  (if (== OtherActor (`GameplayStatics.GetPlayerCharacter` 0))
    (`PlayerCameraManager.RemoveCameraModifier` (`GameplayStatics.GetPlayerCameraManager` 0) (`self.CM`))))

(fn `UserConstructionScript`)