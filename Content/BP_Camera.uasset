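; BP_Camera is a follow camera actor that takes over the first player's view on BeginPlay.
; Each Tick it eases its location toward the player character with an interpolated, swept move.
; While the character moves, the dot product of its velocity direction and world Y drives a smoothed spring arm offset, leading the view sideways along that axis at a fixed raised height.
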(event `self.ReceiveBeginPlay`
  (`PlayerController.SetViewTargetWithBlend` (`GameplayStatics.GetPlayerController` 0) self 0.0 "VTBlend_Linear" 0.0 false))

(event `self.ReceiveTick`
  (params (DeltaSeconds :type "Float (single-precision)"))
  (`self.K2_SetActorLocation` (`KismetMathLibrary.VInterpTo` (`self.K2_GetActorLocation`) (`self.K2_GetActorLocation` (`GameplayStatics.GetPlayerCharacter` 0)) DeltaSeconds 3.0) true)
  (if (> (`KismetMathLibrary.VSize` (`self.GetVelocity` (`GameplayStatics.GetPlayerCharacter` 0))) 0.0)
    ;[1 1 1] Player Rotation based spring arm offset
    (set `SpringArmComponent.TargetOffset` (`KismetMathLibrary.VInterpTo` (`SpringArmComponent.TargetOffset` (`self.SpringArm`)) (+ (* (0.0 200.0 0.0) (`KismetMathLibrary.Dot_VectorVector` (`KismetMathLibrary.Normal` (`self.GetVelocity` (`GameplayStatics.GetPlayerCharacter` 0))) (0.0 1.0 0.0))) (0.0 0.0 150.0)) (`GameplayStatics.GetWorldDeltaSeconds`) 3.0) (`self.SpringArm`))))

(fn `UserConstructionScript`)